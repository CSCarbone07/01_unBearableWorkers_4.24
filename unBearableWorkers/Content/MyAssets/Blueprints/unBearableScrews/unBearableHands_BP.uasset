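; Screw-placing minigame Blueprint that splits roles by player controller ID, showing different screw and floor meshes for each.
; Players 0 and 2 press the face button matching NextButton to animate a screw into place, score and set the rotating stage.
; Players 1 and 3 use movement axes, checked against eight circular stick stages, to drive it down.
; Chained timelines then shift the floor and randomise the next button.
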(event `self.ReceiveBeginPlay`
  (bind _playerid (`self.PlayerID`))
  (bind _initialscrewlocations (`self.InitialScrewLocations`))
  (`parent.ReceiveBeginPlay`)
  (`KismetArrayLibrary.Array_Add` _initialscrewlocations (`SceneComponent.K2_GetComponentLocation` (`self.Screw1`)))
  (`KismetArrayLibrary.Array_Add` _initialscrewlocations (`SceneComponent.K2_GetComponentLocation` (`self.Screw3`)))
  (set `self.Screw2InitialTransform` (`SceneComponent.K2_GetComponentToWorld` (`self.Screw2`)))
  (bind _asplayer_controller (cast `PlayerController` (`self.GetOwner`)))
  (set `self.PlayerID` (`GameplayStatics.GetPlayerControllerID` _asplayer_controller))
  (if (or (== _playerid 1) (== _playerid 3))
    (`SceneComponent.SetVisibility` (`self.Screw2`) false false)
    (else
      (`SceneComponent.SetVisibility` (`self.Floor`) false false)
      (`SceneComponent.SetVisibility` (`self.Screw1`) false false))))

(event `UpdateInstructions`)

(event `InputAxis|MoveForward`
  (params (AxisValue :type "Float (single-precision)"))
  (bind _expectedyaxis (`self.ExpectedYAxis`))
  (bind _expectedxaxis (`self.ExpectedXAxis`))
  (bind _rotationstage (`self.RotationStage`))
  (bind _playerid (`self.PlayerID`))
  (bind (_returnvalue_location _returnvalue_rotation _returnvalue_scale) (`KismetMathLibrary.BreakTransform` (`SceneComponent.GetRelativeTransform` (`self.Screw1`))))
  (bind (_returnvalue_location_2 _returnvalue_rotation_2 _returnvalue_scale_2) (`KismetMathLibrary.BreakTransform` (`SceneComponent.GetRelativeTransform` (`self.Floor`))))
  (if (or (== _playerid 1) (== _playerid 3)) :!label _label
    (if (`self.isRotatingStage`)
      (`KismetSystemLibrary.PrintString` (`KismetStringLibrary.Conv_DoubleToString` AxisValue))
      (switch `int` (`self.RotationStage`)
        (:`0`
          (set `self.ExpectedYAxis` 1.0)
          (set `self.ExpectedXAxis` 0.0))
        (:`1`
          (set `self.ExpectedYAxis` 0.75)
          (set `self.ExpectedXAxis` 0.75))
        (:`2`
          (set `self.ExpectedYAxis` 0.0)
          (set `self.ExpectedXAxis` 1.0))
        (:`3`
          (set `self.ExpectedYAxis` -0.75)
          (set `self.ExpectedXAxis` 0.75))
        (:`4`
          (set `self.ExpectedYAxis` -1.0)
          (set `self.ExpectedXAxis` 0.0))
        (:`5`
          (set `self.ExpectedYAxis` -0.75)
          (set `self.ExpectedXAxis` -0.75))
        (:`6`
          (set `self.ExpectedYAxis` 0.0)
          (set `self.ExpectedXAxis` -1.0))
        (:`7`
          (set `self.ExpectedYAxis` 0.75)
          (set `self.ExpectedXAxis` -0.75)))
      (if (and (`KismetMathLibrary.InRange_FloatFloat` AxisValue (- _expectedyaxis 0.2) (+ _expectedyaxis 0.2)) (`KismetMathLibrary.InRange_FloatFloat` (stale `InputAxis|MoveRight` AxisValue) (- _expectedxaxis 0.2) (+ _expectedxaxis 0.2)))
        (if (== _rotationstage 7)
          (set `self.RotationStage` 0)
          (set `self.isRotatingStage` false)
          (bind (_direction _newtrack_0) (`Timeline|ScrewTime` :!via `PlayFromStart`)
            (:`Update`
              (`SceneComponent.K2_SetRelativeTransform` (`self.Screw1`) (`KismetMathLibrary.TLerp` (`KismetMathLibrary.MakeTransform` _returnvalue_location _returnvalue_rotation _returnvalue_scale) (`KismetMathLibrary.MakeTransform` (- _returnvalue_location (0.0 0.0 15.0)) (struct :`Yaw` -270.0 :`Roll` -180.0) _returnvalue_scale) _newtrack_0) false false))
            (:`Finished`
              (bind (_direction_2 _mapandscrewalpha) (`Timeline|ScrewTimeline` :!via `PlayFromStart`)
                (:`Update`
                  (`SceneComponent.K2_SetRelativeTransform` (`self.Floor`) (`KismetMathLibrary.TLerp` (`KismetMathLibrary.MakeTransform` _returnvalue_location_2 _returnvalue_rotation_2 _returnvalue_scale_2) (`KismetMathLibrary.MakeTransform` (- _returnvalue_location_2 (0.0 -35.0 0.0)) _returnvalue_rotation_2 _returnvalue_scale_2) _mapandscrewalpha) false false))
                (:`Finished`
                  (`SceneComponent.SetVisibility` (`self.Screw1`) false false)
                  (`SceneComponent.K2_SetWorldLocation` (`self.Screw3`) (`|GetArrayItem` (`self.InitialScrewLocations`) 1) false false)
                  (set `self.NextButton` (`KismetMathLibrary.RandomInteger` 4))))))
          (else
            (`/Engine/EditorBlueprintResources/StandardMacros.IncrementInt` _rotationstage)))))))

(event `InputAxis|MoveRight`
  (params (AxisValue :type "Float (single-precision)"))
  (goto _label))

(event `SetExpectedValues`)

(event `self.ReceiveTick`
  (params (DeltaSeconds :type "Float (single-precision)")))

(event `InputAction|cross`
  (params (Key :type "Key Structure"))
  (bind _playerid (`self.PlayerID`))
  (bind (_returnvalue_location _returnvalue_rotation _returnvalue_scale) (`KismetMathLibrary.BreakTransform` (`SceneComponent.K2_GetComponentToWorld` (`self.Screw2`))))
  (:`Pressed`
    (if (== (`self.NextButton`) 0)
      (if (and (or (== _playerid 0) (== _playerid 2)) (not (`self.isRotatingStage`))) :!label _label_2
        (bind (_direction _mapandscrewalpha) (`Timeline|Timeline_0` :!via `PlayFromStart`)
          (:`Update`
            (`SceneComponent.K2_SetRelativeTransform` (`self.Screw2`) (`KismetMathLibrary.TLerp` (`KismetMathLibrary.MakeTransform` _returnvalue_location _returnvalue_rotation _returnvalue_scale) (`KismetMathLibrary.MakeTransform` (`|GetArrayItem` (`self.InitialScrewLocations`)) (struct :`Yaw` 90.0 :`Roll` -180.0) _returnvalue_scale) _mapandscrewalpha) false false))
          (:`Finished`
            (`SceneComponent.K2_SetWorldLocation` (`self.Screw1`) (`|GetArrayItem` (`self.InitialScrewLocations`)) false false)
            (`SceneComponent.K2_SetWorldTransform` (`self.Screw2`) (`self.Screw2InitialTransform`) false false)
            (set `self.isRotatingStage` true)
            (`/Engine/EditorBlueprintResources/StandardMacros.IncrementInt` (`self.Score`))))))))

(event `InputAction|square`
  (params (Key :type "Key Structure"))
  (:`Pressed`
    (if (== (`self.NextButton`) 1)
      (goto _label_2))))

(event `InputAction|triangle`
  (params (Key :type "Key Structure"))
  (:`Pressed`
    (if (== (`self.NextButton`) 2)
      (goto _label_2))))

(event `InputAction|circle`
  (params (Key :type "Key Structure"))
  (:`Pressed`
    (if (== (`self.NextButton`) 3)
      (goto _label_2))))

(fn `UserConstructionScript`
  (`parent.UserConstructionScript`))