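; Game mode for unBearableScrews that sets up local players, their characters and an optional two-screen camera layout.
; On BeginPlay it gathers PlayerStarts and TwoScreenCamera actors, ordering each by a digit parsed from its display name.
; The game instance receives the start points, creates controllers if needed and spawns each player's character.
; It then spawns a WorldHandler to update the screen grid and, with two screens, assigns each controller its camera.
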(event `self.ReceiveBeginPlay`
  (bind _gameinstance_ref (`self.gameInstance_REF`))
  (bind _asmy_game_instance (cast `/Game/MyAssets/Blueprints/myGameInstance` (`GameplayStatics.GetGameInstance`)))
  (set `self.gameInstance_REF` _asmy_game_instance)
  (`self.GetPositionsAndCameras`
    (:`Out`
      (if (not (`/Game/MyAssets/Blueprints/myGameInstance.PlayersWereCreated` _gameinstance_ref))
        (`/Game/MyAssets/Blueprints/myGameInstance.CreateControllers` _gameinstance_ref))
      (`self.SpawnCharacters`)
      (`self.SetScreens`))))

(event `requestSpawn`
  (`/Game/MyAssets/Blueprints/myGameInstance.SpawnCharacter` :`self` (`self.gameInstance_REF`)))

(event `AssignTwoScreenCameras`
  (params (CameraActors :type "Array of /Game/MyAssets/Blueprints/twoScreenCamera_BP Object Reference"))
  (set `self.camerasForTwoScreens` CameraActors))

(fn `SetScreens`
  (bind _camerasfortwoscreens (`self.camerasForTwoScreens`))
  (bind _use2screens (`self.use2Screens`))
  (bind _returnvalue (`|SpawnActorFromClass` "/Game/MyAssets/Blueprints/WorldHandler_BP.WorldHandler_BP_C" (`self.GetTransform`) "Undefined" "OverrideRootScale" self null))
  (`WorldHandler_CPP.updateScreensGrid` _returnvalue _use2screens)
  (if _use2screens
    (`PlayerController.SetViewTargetWithBlend` (`GameplayStatics.GetPlayerController` 0) (`|GetArrayItem` _camerasfortwoscreens) 0.0 "VTBlend_Linear" 0.0 false)
    (`PlayerController.SetViewTargetWithBlend` (`GameplayStatics.GetPlayerController` 1) (`|GetArrayItem` _camerasfortwoscreens 1) 0.0 "VTBlend_Linear" 0.0 false)))

(fn `SpawnCharacters`
  (for (_array_element _array_index) (`self.InitialPositions`)
    (bind _output (`|GetArrayItem` (`self.Character`) _array_index))
    (if (`KismetSystemLibrary.IsValidClass` _output)
      (`/Game/MyAssets/Blueprints/myGameInstance.SpawnCharacter` (`self.gameInstance_REF`) (`GameplayStatics.GetPlayerController` _array_index) _output (`self.GetTransform` _array_element)))))

(fn `UserConstructionScript`)