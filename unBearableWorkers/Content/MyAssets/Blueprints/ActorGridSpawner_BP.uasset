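; Grid spawner actor that fills a box-shaped bound with randomly chosen actor classes, optionally on BeginPlay.
; GridSpawn steps through nested X, Y, Z loops at fixed spacing, applying a density roll and random location, rotation and scale jitter.
; GetRandomActorToSpawn supports weighted picks through ClassBias.
; RotateSpawnLocation rotates positions around the spawner to match its rotation, though the Z loop moves the spawner itself instead of the spawned actor.
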(event `self.ReceiveBeginPlay`
  (if (`self.SpawnOnBeginPlay`)
    (`self.GridSpawn`)))

(fn `GetRandomActorToSpawn`
  (returns (ActorSelectedToSpawn :type "Actor Class Reference"))
  (bind _classbias (`self.classBias`))
  (bind _actorstospawn (`self.ActorsToSpawn`))
  (if (> (`KismetArrayLibrary.Array_Length` _classbias) 0)
    (return (`|GetArrayItem` _actorstospawn (`/Game/MyAssets/Blueprints/myMathFunctions_BL.RandomWithBias` _classbias)))
    (else
      (return (`|GetArrayItem` _actorstospawn (`KismetMathLibrary.RandomInteger` (`KismetArrayLibrary.Array_Length` _actorstospawn)))))))

(fn `GridSpawn`
  (bind (_returnvalue_x _returnvalue_y _returnvalue_z) (`KismetMathLibrary.BreakVector` (`self.K2_GetActorLocation`)))
  (bind _locationrandomness (`self.LocationRandomness`))
  (bind _rotationrandomness (`self.RotationRandomness`))
  (bind _classtospawn (`self.classToSpawn`))
  (bind _scalerandomness (`self.ScaleRandomness`))
  (bind (_boundcorner_x _boundcorner_y _boundcorner_z) (`KismetMathLibrary.BreakVector` (`self.BoundCorner`)))
  (bind _distancebetweenactors (`self.DistanceBetweenActors`))
  (bind _spawns (`self.Spawns`))
  (bind (_out_x _out_y _out_z) (`KismetMathLibrary.BreakVector` (`/Game/MyAssets/Blueprints/myMathFunctions_BL.RandomVectorInRange` (`KismetMathLibrary.NegateVector` _locationrandomness) _locationrandomness)))
  (bind _out (`/Game/MyAssets/Blueprints/myMathFunctions_BL.RandomRotatorInRange` (`KismetMathLibrary.NegateRotator` _rotationrandomness) _rotationrandomness))
  (bind _returnvalue (>= (`self.Density`) (* (`KismetMathLibrary.RandomFloat`) 100.0)))
  (bind _returnvalue_2 (- (`KismetMathLibrary.FTrunc` (/ _boundcorner_y _distancebetweenactors)) 0))
  (bind _returnvalue_3 (`KismetMathLibrary.RandomFloatInRange` (+ (* _scalerandomness -1.0) 1.0) (+ _scalerandomness 1.0)))
  (bind _returnvalue_4 (- (`KismetMathLibrary.FTrunc` (/ _boundcorner_z (`self.DistanceBetweenActors`))) 0))
  (for _index (range (+ (- (`KismetMathLibrary.FTrunc` (/ _boundcorner_x _distancebetweenactors)) 0) 1))
    (bind _output_get (set `self.classToSpawn` (`self.GetRandomActorToSpawn`)))
    (if (`KismetSystemLibrary.IsValidClass` _output_get)
      (if _returnvalue
        (bind _returnvalue_5 (+ _returnvalue_x (* _index (`self.DistanceBetweenActors`))))
        (bind _returnvalue_6 (`|SpawnActorFromClass` _classtospawn (`KismetMathLibrary.MakeTransform` (`KismetMathLibrary.MakeVector` (+ _returnvalue_5 _out_x) (+ _returnvalue_y _out_y) (+ _returnvalue_z _out_z)) _out (`KismetMathLibrary.Conv_DoubleToVector` _returnvalue_3)) "Undefined" "OverrideRootScale" self null))
        (`KismetArrayLibrary.Array_Add` _spawns _returnvalue_6)
        (`/Engine/EditorBlueprintResources/StandardMacros.IsValid` _returnvalue_6
          (:`Is Valid`
            (`self.K2_SetActorLocation` _returnvalue_6 (`self.RotateSpawnLocation` _returnvalue_6) false false))
          (:`Is Not Valid`
            _))))
    (if (>= _returnvalue_2 1)
      (for _index_2 (range 1 (+ _returnvalue_2 1))
        (bind _output_get_2 (set `self.classToSpawn` (`self.GetRandomActorToSpawn`)))
        (if (`KismetSystemLibrary.IsValidClass` _output_get_2)
          (if _returnvalue
            (bind _returnvalue_7 (+ _returnvalue_y (* _index_2 (`self.DistanceBetweenActors`))))
            (bind _returnvalue_8 (`|SpawnActorFromClass` _classtospawn (`KismetMathLibrary.MakeTransform` (`KismetMathLibrary.MakeVector` (+ _returnvalue_5 _out_x) (+ _returnvalue_7 _out_y) (+ _returnvalue_z _out_z)) _out (`KismetMathLibrary.Conv_DoubleToVector` _returnvalue_3)) "Undefined" "OverrideRootScale" self null))
            (`KismetArrayLibrary.Array_Add` _spawns _returnvalue_8)
            (`/Engine/EditorBlueprintResources/StandardMacros.IsValid` _returnvalue_8
              (:`Is Valid`
                (`self.K2_SetActorLocation` _returnvalue_8 (`self.RotateSpawnLocation` _returnvalue_8) false false))
              (:`Is Not Valid`
                _))))
        (if (>= _returnvalue_4 1)
          (for _index_3 (range 1 (+ _returnvalue_4 1))
            (bind _output_get_3 (set `self.classToSpawn` (`self.GetRandomActorToSpawn`)))
            (if (`KismetSystemLibrary.IsValidClass` _output_get_3)
              (if _returnvalue
                (bind _returnvalue_9 (`|SpawnActorFromClass` _classtospawn (`KismetMathLibrary.MakeTransform` (`KismetMathLibrary.MakeVector` (+ _out_x _returnvalue_5) (+ _out_y _returnvalue_7) (+ _out_z (+ _returnvalue_z (* _index_3 (`self.DistanceBetweenActors`))))) _out (`KismetMathLibrary.Conv_DoubleToVector` _returnvalue_3)) "Undefined" "OverrideRootScale" self null))
                (`KismetArrayLibrary.Array_Add` _spawns _returnvalue_9)
                (`/Engine/EditorBlueprintResources/StandardMacros.IsValid` _returnvalue_9
                  (:`Is Valid`
                    (`self.K2_SetActorLocation` (`self.RotateSpawnLocation` _returnvalue_9))))))))))))

(fn `RotateSpawnLocation`
  (params (ActorReference :type "Actor Object Reference"))
  (returns (NewLocation :type "Vector Structure"))
  (bind _returnvalue (`self.K2_GetActorLocation`))
  (return (+ _returnvalue (`KismetMathLibrary.GreaterGreater_VectorRotator` (- (`self.K2_GetActorLocation` ActorReference) _returnvalue) (`self.K2_GetActorRotation`)))))

(fn `UserConstructionScript`)