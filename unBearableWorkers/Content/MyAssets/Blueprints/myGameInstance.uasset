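; Game instance that manages local multiplayer players and the pawns they control.
; It creates extra local players with controllers once, guarded by a flag, and stores starting positions passed to it.
; SpawnCharacter replaces a controller's existing pawn with a given class, then possesses it and targets the view on it.
; DespawnPlayer only destroys the pawn; random-start spawning with a spectator camera sits in unconnected nodes.
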(event `CreateControllers`
  (if (not (`self.PlayersWereCreated`))
    (for _ (range 4)
      (`GameplayStatics.CreatePlayer` -1)
      (set `self.PlayersWereCreated` true))))

(event `RecieveStartingPoints`
  (params (StartingPositions :type "Array of PlayerStart Object Reference"))
  (set `self.StartingPositions` StartingPositions))

(event `SpawnCharacter`
  (params (PlayerController :type "PlayerController Object Reference") (CharacterToSpawn :type "Pawn Class Reference") (SpawningTransform :type "Transform Structure"))
  (bind _returnvalue (`Controller.K2_GetPawn` PlayerController))
  (`/Engine/EditorBlueprintResources/StandardMacros.IsValid` _returnvalue
    (:`Is Valid`
      (`Actor.K2_DestroyActor` _returnvalue)
      (bind _returnvalue_2 (`|SpawnActorFromClass` CharacterToSpawn SpawningTransform "Undefined" "OverrideRootScale" PlayerController null))
      (`Controller.Possess` PlayerController _returnvalue_2)
      (`PlayerController.SetViewTargetWithBlend` PlayerController _returnvalue_2 0.0 "VTBlend_Linear" 0.0 false))))

(event `DespawnPlayer`
  (params (PlayerController :type "PlayerController Object Reference") (ActorToSpawn :type "Actor Class Reference"))
  (bind _returnvalue (`Controller.K2_GetPawn` PlayerController))
  (`/Engine/EditorBlueprintResources/StandardMacros.IsValid` _returnvalue
    (:`Is Valid`
      (`Actor.K2_DestroyActor` _returnvalue))))