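; Blueprint math function library of random helpers for vectors, rotators and weighted index picks.
; The range functions randomize each axis independently between Min and Max, returning three separate floats.
; RandomWithBias rolls once out of 100 and returns the index whose cumulative bias band contains it, so biases act as percentages.
; The older RandomWithBiasOld rerolls per element, taking the first pass or falling back to the last index.
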(fn `RandomRotatorInRange`
  (params (Min :type "Rotator Structure") (Max :type "Rotator Structure"))
  (returns (Out :type "Rotator Structure"))
  (return (`KismetMathLibrary.MakeRotator` (`KismetMathLibrary.RandomFloatInRange` Min_Roll Max_Roll) (`KismetMathLibrary.RandomFloatInRange` Min_Pitch Max_Pitch) (`KismetMathLibrary.RandomFloatInRange` Min_Yaw Max_Yaw))))

(fn `RandomVectorInRange`
  (params (Min :type "Vector Structure") (Max :type "Vector Structure"))
  (returns (Out :type "Vector Structure"))
  (return (`KismetMathLibrary.MakeVector` (`KismetMathLibrary.RandomFloatInRange` Min_X Max_X) (`KismetMathLibrary.RandomFloatInRange` Min_Y Max_Y) (`KismetMathLibrary.RandomFloatInRange` Min_Z Max_Z))))

(fn `RandomWithBias`
  (params (Biases :type "Array of Float (double-precision)"))
  (returns (RandomInt :type Integer))
  (locals (IntResult :type Integer :default 0) (RandomSelection :type "Float (double-precision)") (MinLimit :type "Float (double-precision)") (MaxLimit :type "Float (double-precision)"))
  (set `local.RandomSelection` (* (`KismetMathLibrary.RandomFloat`) 100.0))
  (for (_array_element _array_index) Biases
    (set `local.MinLimit` (`local.MaxLimit`))
    (set `local.MaxLimit` (+ _array_element (`local.MinLimit`)))
    (if (`KismetMathLibrary.InRange_FloatFloat` (`local.RandomSelection`) (`local.MinLimit`) (`local.MaxLimit`))
      (set `local.IntResult` _array_index)))
  (return (`local.IntResult`)))

(fn `RandomWithBiasOld`
  (params (Biases :type "Array of Float (double-precision)"))
  (returns (RandomInt :type Integer))
  (locals (IntResult :type Integer :default -1))
  (for (_array_element _array_index) Biases
    (if (>= _array_element (* (`KismetMathLibrary.RandomFloat`) 100.0))
      (set `local.IntResult` _array_index)
      (break)))
  (if (>= (`local.IntResult`) 0)
    (return (`local.IntResult`))
    (else
      (return (- (`KismetArrayLibrary.Array_Length` Biases) 1)))))