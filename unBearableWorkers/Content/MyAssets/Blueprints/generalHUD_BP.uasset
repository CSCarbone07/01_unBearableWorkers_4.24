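; General HUD Blueprint that puts a countdown-style Timer widget on screen.
; The ShowTimer event creates the widget, stores it, adds it to the viewport and sets its Timer to 30.
; DrawHUD is empty, with leftover unconnected nodes that would print the screen width and draw a 2ndScreen texture at full width and half height.
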(event `self.ReceiveDrawHUD`
  (params (SizeX :type Integer) (SizeY :type Integer)))

(event `ShowTimer`
  (bind _returnvalue (`|CreateWidget` "/Game/MyAssets/Blueprints/Timer.Timer_C"))
  (bind _output_get (set `self.TimerWidget` _returnvalue))
  (`UserWidget.AddToViewport` _output_get 0)
  (set `/Game/MyAssets/Blueprints/Timer.Timer` 30.0 _output_get))

(fn `UserConstructionScript`)